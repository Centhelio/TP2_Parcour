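; BP_DeathZone is a trigger volume that changes the player's health when their character overlaps its Collision component.
; It reaches the ACHealth component on BP_PlayerState through the overlapping BP_ThirdPersonCharacter.
; The sign of HealthChangeAmount selects damage or healing.
; A 2D death scream then plays in either case, as its branch condition is fixed to true.
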(event OnComponentBeginOverlap(Collision)
  (params (OverlappedComponent :type Primitive%20Component%20Object%20Reference) (OtherActor :type Actor%20Object%20Reference) (OtherComp :type Primitive%20Component%20Object%20Reference) (OtherBodyIndex :type Integer) (bFromSweep :type Boolean) (SweepResult :type Hit%20Result%20Structure%20%28by%20ref%29))
  (bind _asbp_third_person_character (Utilities|Casting|CastToBP_ThirdPersonCharacter OtherActor))
  (bind _asbp_player_state (Utilities|Casting|CastToBP_PlayerState (Variables|/Script/Engine.Pawn|GetPlayerState _asbp_third_person_character)))
  (if (< (Variables|Default|GetHealthChangeAmount) 0.0)
    (Default|TakeDamage (Variables|/Game/Game/Blueprints/PlayerStates/BP_PlayerState.BP_PlayerState_C|GetAC_Health _asbp_player_state) (Math|Float|Absolute(Float) (Variables|Default|GetHealthChangeAmount)))
    (else
      (Default|GainHealth (Variables|/Game/Game/Blueprints/PlayerStates/BP_PlayerState.BP_PlayerState_C|GetAC_Health _asbp_player_state) (Math|Float|Absolute(Float) (Variables|Default|GetHealthChangeAmount)))))
  (if true
    (Audio|PlaySound2D "/Game/Game/Audio/SFX/male-death-scream-horror-352706.male-death-scream-horror-352706" 1.0 1.0 0.0 0 0)))

(fn ConstructionScript)