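; AC_Health is an actor component that tracks an owner's health and death state.
; TakeDamage, GainHealth and ResetHealth events all route through UpdateHealthAndNotify, with damage and healing ignored once dead.
; That function clamps health between zero and MaxHealth, broadcasts OnHealthChanged, then sets IsDead and fires OnDeath when health reaches zero.
; ResetHealth clears the dead flag and restores full health, allowing revival.
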(event EventTakeDamage
  (params (DamageAmount :type Float%20%28double-precision%29))
  (if (not (Variables|Default|GetIsDead))
    (CallFunction|UpdateHealthandNotify (- (Variables|Default|GetCurrentHealth) DamageAmount))))

(event EventGainHealth
  (params (Health :type Float%20%28double-precision%29))
  (if (not (Variables|Default|GetIsDead))
    (CallFunction|UpdateHealthandNotify (+ (Variables|Default|GetCurrentHealth) Health))))

(event EventResetHealth
  (Variables|Default|SetIsDead false)
  (CallFunction|UpdateHealthandNotify (Variables|Default|GetMaxHealth)))

(fn UpdateHealthandNotify
  (params (NewHealthValue :type Float%20%28double-precision%29))
  ;[0.15 0.15 0.15 0.5] Mettre à jour les variables de AC_Health
  (bind _output_get (Variables|Default|SetCurrentHealth (Math|Float|Clamp(Float) NewHealthValue 0.0 (Variables|Default|GetMaxHealth))))
  (Default|CallOnHealthChanged _output_get (Variables|Default|GetMaxHealth))
  (if (<= (Variables|Default|GetCurrentHealth) 0.0)
    (Variables|Default|SetIsDead true)
    (Default|CallOnDeath)
    (else
      (Variables|Default|SetIsDead false))))