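; Interaction-system grid that moves vertically when activated and returns when deactivated.
; BeginPlay binds the activate and deactivate events to handlers that play one timeline from the start or reverse it from the end.
; The timeline's Percentage drives the Grid component's relative height, leaving X and Y unchanged.
; The ActivateFunc and DeactivateFunc functions do nothing, as all logic lives in the event graph.
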(event Custom|CallFunction
  (bind _grid (Variables|Default|GetGrid))
  (bind _relativelocation (Variables|/Script/Engine.SceneComponent|GetRelativeLocation _grid))
  (bind (_x _y) (Math|Vector|BreakVector _relativelocation))
  (bind _percentage (Timeline|Timeline PlayFromStart)
    (:Update
      (Transformation|SetRelativeLocation _grid (Math|Vector|MakeVector _x _y (* _percentage 3.5e+02)) false false))))

(event Custom|CallDeactivate
  (bind _grid (Variables|Default|GetGrid))
  (bind _relativelocation (Variables|/Script/Engine.SceneComponent|GetRelativeLocation _grid))
  (bind (_x _y) (Math|Vector|BreakVector _relativelocation))
  (bind _percentage (Timeline|Timeline ReverseFromEnd)
    (:Update
      (Transformation|SetRelativeLocation _grid (Math|Vector|MakeVector _x _y (* _percentage 3.5e+02)) false false))))

(event EventBeginPlay
  (EventDispatchers|BindEventtoActivate (delegate Custom|CallFunction))
  (EventDispatchers|BindEventtoDeactivate (delegate Custom|CallDeactivate)))

(event Collision|EventActorBeginOverlap
  (params (OtherActor :type Actor%20Object%20Reference)))

(event EventTick
  (params (DeltaSeconds :type Float%20%28single-precision%29)))

(fn ConstructionScript)

(fn ActivateFunc)

(fn DeactivateFunc)