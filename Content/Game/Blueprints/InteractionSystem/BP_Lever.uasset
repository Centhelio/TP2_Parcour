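; BP_Lever is a one-shot interactable lever in the interaction system.
; Its Interact event sets an Activated flag that blocks repeat use, then plays the Animation timeline.
; Each timeline update subtracts the track value from the Cylinder's current relative Z, so the offset accumulates rather than interpolating from a start position.
; A 2D gear noise also fires on every update, not once per activation.
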(event EventBeginPlay)

(event Collision|EventActorBeginOverlap
  (params (OtherActor :type Actor%20Object%20Reference)))

(event EventTick
  (params (DeltaSeconds :type Float%20%28single-precision%29)))

(event EventInteract
  (if (not (Variables|Default|GetActivated))
    (Variables|Default|SetActivated true)
    (bind _newtrack (Timeline|Animation Play)
      (:Update
        (Transformation|SetRelativeLocation (Variables|Default|GetCylinder) (+ (Math|Vector|MakeVector 0.0 0.0 (* _newtrack -1.0)) (Variables|/Script/Engine.SceneComponent|GetRelativeLocation (Variables|Default|GetCylinder))) false false)
        (Audio|PlaySound2D "/Game/Game/Audio/SFX/gear_noise-427806.gear_noise-427806" 1.0 1.0 0.0 0 0)))))

(fn ConstructionScript)