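; Grille (gate) actor in the interaction system that slides its Grid component vertically when activated or deactivated.
; On BeginPlay it binds its handlers to the Activate and Deactivate events.
; Activation plays a Timeline from the start and deactivation reverses it from the end, with the Timeline's percentage driving the Grid's relative height.
; Both always restart from an endpoint, so interrupting a move makes the grid jump.
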(event Custom|CallActive
  (bind _grid (Variables|Default|GetGrid))
  (bind _relativelocation (Variables|/Script/Engine.SceneComponent|GetRelativeLocation _grid))
  (bind (_x _y) (Math|Vector|BreakVector _relativelocation))
  (bind _percentage (Timeline|Timeline PlayFromStart)
    (:Update
      (Transformation|SetRelativeLocation _grid (Math|Vector|MakeVector _x _y (* _percentage 3e+02)) false false))))

(event Custom|calDeactive
  (bind _grid (Variables|Default|GetGrid))
  (bind _relativelocation (Variables|/Script/Engine.SceneComponent|GetRelativeLocation _grid))
  (bind (_x _y) (Math|Vector|BreakVector _relativelocation))
  (bind _percentage (Timeline|Timeline ReverseFromEnd)
    (:Update
      (Transformation|SetRelativeLocation _grid (Math|Vector|MakeVector _x _y (* _percentage 3e+02)) false false))))

(event EventBeginPlay
  (EventDispatchers|BindEventtoActivate (delegate Custom|CallActive))
  (EventDispatchers|BindEventtoDeactivate (delegate Custom|calDeactive)))

(fn ConstructionScript)