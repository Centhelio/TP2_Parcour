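; BP_EndFlag is an end-of-level flag that lets the player finish the level and load the next map named by WhatLvl.
; Overlap by BP_ThirdPersonCharacter reveals its initially hidden Widget and enables interaction; no end-overlap handler reverses this.
; The flag receives player 0's input directly, so Interact then displays WBP_MessageVictoire and opens that level after a short delay.
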(event OnComponentBeginOverlap(collision)
  (params (OverlappedComponent :type Primitive%20Component%20Object%20Reference) (OtherActor :type Actor%20Object%20Reference) (OtherComp :type Primitive%20Component%20Object%20Reference) (OtherBodyIndex :type Integer) (bFromSweep :type Boolean) (SweepResult :type Hit%20Result%20Structure%20%28by%20ref%29))
  (Utilities|Casting|CastToBP_ThirdPersonCharacter OtherActor)
  (Rendering|SetVisibility (Variables|Default|GetWidget) true false)
  (Variables|Default|SetCanInteract true))

(event EventBeginPlay
  (Rendering|SetVisibility (Variables|Default|GetWidget) false false)
  (Input|EnableInput (Game|GetPlayerController 0)))

(event Input|ActionEvents|InputActionInteract
  (params (Key :type Key%20Structure :default "None"))
  (:Pressed
    (if (Variables|Default|GetCanInteract)
      (bind _returnvalue (UserInterface|CreateWidget "/Game/Game/UI/WBP_MessageVictoire.WBP_MessageVictoire_C"))
      (UserInterface|Viewport|AddtoViewport _returnvalue 0)
      (Utilities|FlowControl|Delay 3.0)
      (Game|OpenLevel(byName) (Variables|Default|GetWhatLvl)))))

(fn ConstructionScript)